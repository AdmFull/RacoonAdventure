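; Player character Blueprint whose graph keeps the health and stamina bars of the player HUD up to date.
; Every Tick, it casts the current game mode's active widget to BPPlayerGUI.
; If the game instance held by its CMComp component is valid, it polls health and stamina percentages from it and sets both progress bars directly.
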(event `self.ReceiveTick`
  (params (DeltaSeconds :type "Float (single-precision)"))
  (bind _cgigameinstance (`RA_CharacterMovementComponent.cgiGameInstance` (`self.CMComp`)))
  (bind _returnvalue (`self.GetCurrentGamemode`))
  (bind _asbpplayer_gui (cast `/Game/Game/GUI/BPPlayerGUI` (`RacoonAdventureGameMode.CurrentWidget` _returnvalue)))
  (if (`KismetSystemLibrary.IsValid` _cgigameinstance)
    (`|ExecutionSequence`
      (:`then_0`
        (bind _returnvalue_2 (`RacoonAdventureGameInstance.GetPlayerHPPerc` _cgigameinstance))
        (`ProgressBar.SetPercent` (`/Game/Game/GUI/BPPlayerGUI.pbHealth` _asbpplayer_gui) _returnvalue_2))
      (:`then_1`
        (bind _returnvalue_3 (`RacoonAdventureGameInstance.GetPlayerStaminaPerc` _cgigameinstance))
        (`ProgressBar.SetPercent` (`/Game/Game/GUI/BPPlayerGUI.pbStamina` _asbpplayer_gui) _returnvalue_3)))))

(fn `UserConstructionScript`)