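; Main character Blueprint for Racoon Adventure that keeps the player HUD's health, mana and stamina bars up to date.
; Every Tick it casts to the game mode's current widget as the player GUI and to the game instance.
; It then copies the instance's HP, mana and stamina percentages into the matching progress bars, polling each frame rather than reacting to change events.
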(event `self.ReceiveTick`
  (params (DeltaSeconds :type "Float (single-precision)"))
  (bind _asmy_racoon_adventure_game_mode (cast `/Game/Game/GameLogic/MyRacoonAdventureGameMode` (`GameplayStatics.GetGameMode`)))
  (bind _asbpplayer_gui (cast `/Game/Game/GUI/BPPlayerGUI` (`RacoonAdventureGameMode.CurrentWidget` _asmy_racoon_adventure_game_mode)))
  (bind _asbpracoon_adventure_game_instance (cast `/Game/Game/GameLogic/BPRacoonAdventureGameInstance` (`GameplayStatics.GetGameInstance`)))
  (`|ExecutionSequence`
    (:`then_0`
      (bind _returnvalue (`RacoonAdventureGameInstance.GetPlayerHPPerc` _asbpracoon_adventure_game_instance))
      (`ProgressBar.SetPercent` (`/Game/Game/GUI/BPPlayerGUI.pbHealth` _asbpplayer_gui) _returnvalue))
    (:`then_1`
      (bind _returnvalue_2 (`RacoonAdventureGameInstance.GetPlayerManaPerc` _asbpracoon_adventure_game_instance))
      (`ProgressBar.SetPercent` (`/Game/Game/GUI/BPPlayerGUI.pbMana` _asbpplayer_gui) _returnvalue_2))
    (:`then_2`
      (bind _returnvalue_3 (`RacoonAdventureGameInstance.GetPlayerStaminaPerc` _asbpracoon_adventure_game_instance))
      (`ProgressBar.SetPercent` (`/Game/Game/GUI/BPPlayerGUI.pbStamina` _asbpplayer_gui) _returnvalue_3))))

(fn `UserConstructionScript`)